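; BP_FallingPlatform is a platform actor, named as a falling platform, that resets after the player touches it.
; BeginPlay saves the Cube's world transform and gives it a random color material from nine options.
; When the player overlaps the Box, two chained delays run, then Cube physics is switched off and it teleports to the saved transform.
; The graph contains no step that enables physics to start a fall.
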(event `self.ReceiveBeginPlay`
  (set `self.DefaultTransform` (`SceneComponent.K2_GetComponentToWorld` (`self.Cube`)))
  (`PrimitiveComponent.SetMaterial` (`self.Cube`) 0 (select `int` (`KismetMathLibrary.RandomIntegerInRange` 0 8) :`0` "/Game/Materials/M_Black.M_Black" :`1` "/Game/Materials/M_Blue.M_Blue" :`2` "/Game/Materials/M_Brown.M_Brown" :`3` "/Game/Materials/M_Green.M_Green" :`4` "/Game/Materials/M_Orange.M_Orange" :`5` "/Game/Materials/M_Purple.M_Purple" :`6` "/Game/Materials/M_Red.M_Red" :`7` "/Game/Materials/M_White.M_White" :`8` "/Game/Materials/M_Yellow.M_Yellow" :!type "MaterialInterface Object Reference")))

(event `self.Box.OnComponentBeginOverlap`
  (params (OverlappedComponent :type "PrimitiveComponent Object Reference") (OtherActor :type "Actor Object Reference") (OtherComp :type "PrimitiveComponent Object Reference") (OtherBodyIndex :type Integer) (bFromSweep :type Boolean) (SweepResult :type "HitResult Structure (by ref)"))
  (bind _cube (`self.Cube`))
  (if (== OtherActor (`GameplayStatics.GetPlayerCharacter` 0))
    (`KismetSystemLibrary.Delay` 1.0)
    (`KismetSystemLibrary.Delay` 5.0)
    (`PrimitiveComponent.SetSimulatePhysics` _cube false)
    (`SceneComponent.K2_SetWorldTransform` _cube (`self.DefaultTransform`) false true)))

(fn `UserConstructionScript`)